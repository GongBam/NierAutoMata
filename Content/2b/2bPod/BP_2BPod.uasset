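; BP_2BPod is a companion pawn that follows the BP_Character actor around the level.
; Each Tick looks up the character and runs 2BFollow, which issues AI MoveTo toward it at 400 units or more away.
; When closer, it halts by targeting itself.
; Both branches also re-invoke 2BFollow through a short Delay, alongside the per-frame calls from Tick.
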(event `self.ReceiveTick`
  (params (DeltaSeconds :type "Float (single-precision)"))
  (bind _returnvalue (`GameplayStatics.GetActorOfClass` "/Game/2b/TEST/BP_Character.BP_Character_C"))
  (set `self.Char Ref` _returnvalue)
  (`self.2B Follow`))

(event `2B Follow`
  (if (>= (`self.GetDistanceTo` (`self.Char Ref`)) 400.0)
    (`|AIMoveTo` self (0.0 0.0 0.0) (`self.Char Ref`)
      (:`then`
        _))
    (else
      (`|AIMoveTo` self (0.0 0.0 0.0) self
        (:`then`
          _))))
  (`KismetSystemLibrary.Delay` 0.2)
  (`self.2B Follow`))

(fn `UserConstructionScript`)