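; Actor component that holds the health and stamina stats for 2B, the player character.
; Health functions adjust the values and push the ratio to the player HUD's health bar; increases clamp to max, and DecreaseHealth returns whether health is depleted.
; Stamina functions have no HUD update, and DecreaseStamina checks and overwrites CurrentHealth with unchanged CurrentStamina.
; IncreaseMaxHealth adds zero, so the maximum never changes, and Tick and BeginPlay are empty.
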(fn `Decrease Health`
  (params (Damage :type "Float (double-precision)"))
  (returns (`Is Player Dead?` :type Boolean))
  (if (not (<= (`self.Current Health`) 0.0))
    (bind _output_get (set `self.Current Health` (- (`self.Current Health`) Damage)))
    (`ProgressBar.SetPercent` (`/Game/2b/UI/WB_HUD.HealthBar` (`/Game/2b/BP_PlayerC.HUD Widget` (`self.Player Character BP`))) (/ _output_get (`self.MaxHealth`)))
    (if (<= (`self.Current Health`) 0.0)
      _
      (else
        (return false))))
  (return true))

(fn `Decrease Stamina`
  (returns (`Not Stamina Left` :type Boolean))
  (if (not (<= (`self.Current Health`) 0.0))
    (set `self.Current Health` (- (`self.Current Stamina`) 0.0))
    (if (<= (`self.Current Health`) 0.0)
      _
      (else
        (return false))))
  (return true))

(fn `Increase Health`
  (params (`Added Health` :type "Float (double-precision)"))
  (set `self.Current Health` (+ (`self.Current Health`) `Added Health`))
  (if (> (`self.Current Health`) (`self.MaxHealth`))
    (set `self.Current Health` (`self.MaxHealth`)))
  (`ProgressBar.SetPercent` (`/Game/2b/UI/WB_HUD.HealthBar` (`/Game/2b/BP_PlayerC.HUD Widget` (`self.Player Character BP`))) (/ (`self.Current Health`) (`self.MaxHealth`))))

(fn `Increase Max Health`
  (set `self.MaxHealth` (+ (`self.MaxHealth`) 0.0))
  (`ProgressBar.SetPercent` (`/Game/2b/UI/WB_HUD.HealthBar` (`/Game/2b/BP_PlayerC.HUD Widget` (`self.Player Character BP`))) (/ (`self.Current Health`) (`self.MaxHealth`))))

(fn `Increase Max Stamina`
  (params (`Added Stamina` :type "Float (double-precision)"))
  (set `self.Max Stamina` (+ (`self.Max Stamina`) `Added Stamina`)))

(fn `Increase Stamina`
  (params (B :type "Float (double-precision)"))
  (set `self.Current Stamina` (+ (`self.Current Stamina`) B))
  (if (> (`self.Current Stamina`) (`self.Max Stamina`))
    (set `self.Current Stamina` (`self.Max Stamina`))))