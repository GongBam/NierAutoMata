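; 9S test companion character that follows the player and fights BP_ADAM with thrown and melee sword attacks.
; Tick drives AI MoveTo toward the player or a nearby enemy, favoring a distant player, while IsFollowing is false.
; PawnSensing turns it toward the enemy, choosing throw or slash montages by distance.
; SwordStarting and GangGong events spawn projectile actors, briefly hide the mesh, and track a throw counter that switches the ranged montage.
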(event `Follow Enemy`
  ;[1 1 1] 에너미가 가까우면 에너미 따라, 아군이 멀어지면 아군따라가기
  (if (`self.IsFollowing?`)
    _
    (elif (<= (`self.GetDistanceTo` (`self.Enermy REF`)) 700.0)
      (if (>= (`self.GetDistanceTo` (`self.Char REF`)) 800.0)
        (`|AIMoveTo` self (0.0 0.0 0.0) (`self.Char REF`))
        (else
          (`|AIMoveTo` self (0.0 0.0 0.0) (`self.Enermy REF`)
            (:`then`
              (if (< (`self.GetDistanceTo` (`self.Enermy REF`)) 500.0)
                (`MovementComponent.StopMovementImmediately` (`self.CharacterMovement`))
                (`KismetSystemLibrary.Delay` 0.1)
                (`self.Follow Enemy`)))))))))

(event `self.ReceiveTick`
  (params (DeltaSeconds :type "Float (single-precision)"))
  ;[1 1 1] 플레이어를 따라 갈까요? 에너미를 따라갈까요?
  (`|ExecutionSequence`
    (:`then_0`
      (bind _asbp_character (cast `/Game/2b/TEST/BP_Character` (`GameplayStatics.GetPlayerCharacter` 0)))
      (set `self.Char REF` _asbp_character)
      (`self.Follow Player`))
    (:`then_1`
      (bind _returnvalue (`GameplayStatics.GetActorOfClass` "/Game/ConvertToC++/FUCK/BP_ADAM.BP_ADAM_C"))
      (set `self.Enermy REF` _returnvalue)
      (`self.Follow Enemy`))))

(event `Follow Player`
  ;[1 1 1] 아군따라가기
  (if (not (`self.IsFollowing?`))
    (if (>= (`self.GetDistanceTo` (`self.Char REF`)) 300.0)
      (`|AIMoveTo` self (0.0 0.0 0.0) (`self.Char REF`)
        (:`then`
          _))
      (else
        (`|AIMoveTo` self (0.0 0.0 0.0) self
          (:`then`
            _))))
    (`KismetSystemLibrary.Delay` 0.1)
    (`self.Follow Enemy`)))

(event `self.PawnSensing.OnSeePawn`
  (params (Pawn :type "Pawn Object Reference"))
  (if (`self.ActorHasTag` Pawn "Enermy")
    (bind _asbp_adam (cast `/Game/ConvertToC++/FUCK/BP_ADAM` Pawn))
    (`KismetSystemLibrary.Delay` 0.1)
    (`self.K2_SetActorRotation` (`KismetMathLibrary.FindLookAtRotation` (`self.K2_GetActorLocation`) (`self.K2_GetActorLocation` _asbp_adam)))
    (if (> (`self.GetDistanceTo` _asbp_adam) 400.0)
      (`self.Throwing`)
      (set `self.IsFollowing?` true)
      (else
        (`self.draw Swoard`)
        (set `self.IsFollowing?` true)))))

(event `GangGong`
  (`|SpawnActorFromClass` "/Game/9S/9sTest/Blueprint/BP_GangGong.BP_GangGong_C" (`KismetMathLibrary.MakeTransform` (+ (`self.K2_GetActorLocation`) (100.0 0.0 0.0))) "AlwaysSpawn" "MultiplyWithRoot" null null)
  (`SceneComponent.SetVisibility` (`self.meshComp`) false false)
  (set `self.Is Throwing?` false)
  (`KismetSystemLibrary.Delay` 2.0)
  (`SceneComponent.SetVisibility` (`self.meshComp`) true false)
  (`KismetSystemLibrary.Delay` 2.0)
  (set `self.Is Throwing?` true)
  (set `self.Already` 0)
  (set `self.IsAttaking?` false)
  (`KismetSystemLibrary.Delay` 1.0)
  (set `self.IsFollowing?` false))

(event `Throwing`
  (if (`self.Is Throwing?`)
    (if (not (`self.IsAttaking?`))
      (set `self.IsAttaking?` true)
      (if (== (`self.Already`) 2)
        (`self.PlayAnimMontage` "/Game/9S/9sTest/Animation/Montage/Thrust_Slash_Montage.Thrust_Slash_Montage")
        (else
          ;[1 1 1] 검발사
          (`self.PlayAnimMontage` "/Game/9S/9sTest/Animation/Montage/Frisbee_Throw_Montage.Frisbee_Throw_Montage"))))))

(event `SwordStarting`
  ;[1 1 1] 검발사
  (`|SpawnActorFromClass` "/Game/9S/9sTest/Blueprint/BP_Weapon.BP_Weapon_C" (`KismetMathLibrary.MakeTransform` (+ (`self.K2_GetActorLocation`) (100.0 0.0 0.0))) "AlwaysSpawn" "MultiplyWithRoot" null null)
  (`SceneComponent.SetVisibility` (`self.meshComp`) false false)
  (set `self.Is Throwing?` false)
  (`KismetSystemLibrary.Delay` 1.0)
  (`SceneComponent.SetVisibility` (`self.meshComp`) true false)
  (`KismetSystemLibrary.Delay` 1.0)
  (set `self.Is Throwing?` true)
  (bind _output_get (set `self.Already` (+ (`self.Already`) 1)))
  (`KismetSystemLibrary.PrintString` (`KismetStringLibrary.Conv_IntToString` _output_get))
  (set `self.IsAttaking?` false)
  (`KismetSystemLibrary.Delay` 1.0)
  (set `self.IsFollowing?` false))

(event `draw Swoard`
  (if (`self.DrawSwoard?`)
    (if (not (`self.IsAttaking?`))
      (set `self.IsAttaking?` true)
      (bind _returnvalue (`self.PlayAnimMontage` "/Game/9S/9sTest/Animation/Montage/SlashSlashSlash.SlashSlashSlash" 1.0 "None"))
      (`KismetSystemLibrary.Delay` _returnvalue)
      (set `self.IsAttaking?` false)
      (`KismetSystemLibrary.Delay` 1.0)
      (set `self.IsFollowing?` false))
    (elif (not (`self.IsAttaking?`))
      (set `self.IsAttaking?` true)
      (bind _returnvalue_2 (`self.PlayAnimMontage` "/Game/9S/9sTest/Animation/Montage/DrawSwoard.DrawSwoard" 1.0 "None"))
      (`KismetSystemLibrary.Delay` _returnvalue_2)
      (bind _returnvalue_3 (`self.PlayAnimMontage` "/Game/9S/9sTest/Animation/Montage/SlashSlashSlash.SlashSlashSlash" 1.0 "None"))
      (`KismetSystemLibrary.Delay` _returnvalue_3)
      (set `self.IsAttaking?` false)
      (`KismetSystemLibrary.Delay` 1.0)
      (set `self.IsFollowing?` false))))

(fn `UserConstructionScript`)