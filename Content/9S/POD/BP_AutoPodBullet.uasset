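; BP_AutoPodBullet is the projectile for the auto pod, built to deactivate rather than destroy itself when its flight ends.
; On a component hit it spawns an impact particle and a short-lived FS_MasterField, triggered with a radial magnitude to apply a field effect at the impact.
; EndLaunch then hides the bullet, disables collision and movement, clears its end-launch timer and broadcasts OnEnd with itself.
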(event `self.autopodbullet.OnComponentHit`
  (params (HitComponent :type "PrimitiveComponent Object Reference") (OtherActor :type "Actor Object Reference") (OtherComp :type "PrimitiveComponent Object Reference") (NormalImpulse :type "Vector Structure") (Hit :type "HitResult Structure (by ref)"))
  (bind (_bblockinghit _binitialoverlap _time _distance _location _impactpoint) (`GameplayStatics.BreakHitResult` Hit))
  (bind (_returnvalue_location _returnvalue_rotation) (`KismetMathLibrary.BreakTransform` (`KismetMathLibrary.Conv_VectorToTransform` _impactpoint)))
  (`GameplayStatics.SpawnEmitterAtLocation` "/Game/Pod/VFX/P_Impact.P_Impact" _location)
  (bind _returnvalue (`|SpawnActorFromClass` "/Engine/EditorResources/FieldNodes/FS_MasterField.FS_MasterField_C" (`KismetMathLibrary.MakeTransform` _location _returnvalue_rotation) "Undefined" "MultiplyWithRoot" null null))
  (set `/Engine/EditorResources/FieldNodes/FS_MasterField.ActivationType` "NewEnumerator4" _returnvalue)
  (set `/Engine/EditorResources/FieldNodes/FS_MasterField.FieldLifespan` 0.1 _returnvalue)
  (set `/Engine/EditorResources/FieldNodes/FS_MasterField.Radial Magnitude` 10.0 _returnvalue)
  (`/Engine/EditorResources/FieldNodes/FS_MasterField.CE_Trigger` _returnvalue)
  (`self.EndLaunch`))

(fn `EndLaunch`
  (`SceneComponent.SetVisibility` (`self.autopodbullet`) false false)
  (`ActorComponent.Deactivate` (`self.ProjectileMovement`))
  (set `self.IsLaunched` false)
  (`PrimitiveComponent.SetCollisionEnabled` (`self.autopodbullet`) "NoCollision")
  (`KismetSystemLibrary.K2_ClearAndInvalidateTimerHandle` (`self.EndLauchTimer`))
  (`self.OnEnd` self))

(fn `UserConstructionScript`)